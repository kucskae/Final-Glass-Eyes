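; AI for a doll character that patrols, chases seen characters and responds to a trigger raised by the player.
; PawnSensing starts a chase, clearing its Seen flag only if that move fails.
; Tick alternates through a looping MultiGate between moving to BoxTrigger when the player's TrigOn is true and a delayed three-target patrol, gated by Seen, Moving and Triggered flags.
; A random navmesh roaming branch is left unconnected.
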(event OnSeePawn(PawnSensing)
  (params (Pawn :type Pawn%20Object%20Reference))
  (bind _ascharacter (Utilities|Casting|CastToCharacter Pawn))
  (Variables|Default|SetSeen true)
  (AI|AIMoveTo self "0, 0, 0" _ascharacter 5.0 false
    (:OnFail
      (Variables|Default|SetSeen false))))

(event EventTick
  (params (DeltaSeconds :type Float%20%28single-precision%29))
  (Utilities|FlowControl|MultiGate false true -1
    (:Out%200
      (bind _trig (Default|TrigOn? (Variables|Default|GetPlayerChar)))
      (if _trig
        (Variables|Default|SetTriggered true)
        (AI|AIMoveTo self "0, 0, 0" (Variables|Default|GetBoxTrigger) 5.0 false
          (:then
            (Variables|Default|SetTriggered true))
          (:OnSuccess
            (Variables|Default|SetTriggered false :!label _label))
          (:OnFail
            (goto _label)))))
    (:Out%201
      (Utilities|FlowControl|Delay 1.0)
      (if (not (Variables|Default|GetSeen))
        (if (not (Variables|Default|GetMoving))
          (if (not (Variables|Default|GetTriggered))
            (AI|AIMoveTo self "0, 0, 0" (Variables|Default|GetTarget1) 5.0 false
              (:OnSuccess
                (Variables|Default|SetMoving true)
                (AI|AIMoveTo self "0, 0, 0" (Variables|Default|GetTarget2) 5.0 false
                  (:OnSuccess
                    (AI|AIMoveTo self "0, 0, 0" (Variables|Default|GetTarget3) 5.0 false
                      (:OnSuccess
                        _)
                      (:OnFail
                        _))
                    (Variables|Default|SetMoving false))
                  (:OnFail
                    (Variables|Default|SetMoving false))))
              (:OnFail
                (Variables|Default|SetMoving false)))))))))

(fn ConstructionScript)